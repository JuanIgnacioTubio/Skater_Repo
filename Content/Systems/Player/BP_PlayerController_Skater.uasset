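; Player controller for the skater character that relays movement state changes to the HUD.
; On BeginPlay it caches the controlled pawn as the skater character and the HUD as BP_HUD_Skater.
; Walking, riding, jumping and falling events in a separate HUD graph each forward to the matching function on the cached HUD.
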(event EventBeginPlay
  (Variables|Default|SetPlayerPawn (.AsSkater%20BGSCharacter (Utilities|Casting|CastToSkater_BGSCharacter (Pawn|GetControlledPawn))))
  (Variables|Default|SetHUDClass (.AsBP%20HUD%20Skater (Utilities|Casting|CastToBP_HUD_Skater (HUD|GetHUD)))))

(event Custom|SetStateFalling
  (Default|SetStateFalling (Variables|Default|GetHUDClass)))

(event Custom|SetStateWalking
  (Default|SetStateWalking (Variables|Default|GetHUDClass)))

(event Custom|SetStateRiding
  (Default|SetStateRiding (Variables|Default|GetHUDClass)))

(event Custom|SetStateJumping
  (Default|SetStateJumping (Variables|Default|GetHUDClass)))

(fn ConstructionScript)