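; Game instance for the skater game that holds player progress across levels: unlocked levels, per-level high scores and play time.
; On Init it loads save slot "0" into its variables, or creates a new save object if none exists.
; Events track total and current-stage play time and record combo scores beating MaxComboScore as the stage's high score.
; SaveGame writes the variables back to the slot, and DeleteSaveGame removes it.
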(event Custom|SaveGame
  (bind _savegamefile (Variables|Internal|GetSaveGameFile))
  (Variables|/Game/Systems/BP_SaveGame_Skater.BP_SaveGame_Skater_C|SetLevelsUnlocked _savegamefile (Variables|Persistence|GetLevelsUnlocked))
  (Variables|/Game/Systems/BP_SaveGame_Skater.BP_SaveGame_Skater_C|SetTotalTimePlayed _savegamefile (Variables|Persistence|GetTotalTimePlayed))
  (Variables|/Game/Systems/BP_SaveGame_Skater.BP_SaveGame_Skater_C|SetLevelTimePlayed _savegamefile (Variables|Persistence|GetLevelTimePlayed))
  (Variables|/Game/Systems/BP_SaveGame_Skater.BP_SaveGame_Skater_C|SetLevelHighScore _savegamefile (Variables|Persistence|GetLevelHighScore))
  (SaveGame|SaveGametoSlot _savegamefile "0"))

(event Custom|DeleteSaveGame
  (SaveGame|DeleteGameinSlot "0"))

(event Custom|SetLevelHighScore
  (params (TotalComboScore :type Float%20%28double-precision%29))
  (if (> TotalComboScore (Variables|Default|GetMaxComboScore))
    (bind _output_get (Variables|Default|SetMaxComboScore TotalComboScore))
    (Utilities|Array|SetArrayElem (Variables|Persistence|GetLevelHighScore) (Variables|Default|GetCurrentStage) _output_get true)))

(event Custom|TickTimePlayed
  (params (DeltaTime :type Float%20%28double-precision%29))
  (bind _leveltimeplayed (Variables|Persistence|GetLevelTimePlayed))
  (Variables|Persistence|SetTotalTimePlayed (+ (Variables|Persistence|GetTotalTimePlayed) (Math|Timespan|FromSeconds DeltaTime)))
  (Utilities|Array|SetArrayElem _leveltimeplayed (Variables|Default|GetCurrentStage) (+ (Utilities|Array|Get(acopy) _leveltimeplayed (Variables|Default|GetCurrentStage)) (Math|Timespan|FromSeconds DeltaTime)) true))

(event EventInit
  (bind _returnvalue (SaveGame|DoesSaveGameExist "0"))
  (if _returnvalue
    (bind _returnvalue_2 (SaveGame|LoadGamefromSlot "0"))
    (bind _output_get (Variables|Internal|SetSaveGameFile (.AsBP%20Save%20Game%20Skater (Utilities|Casting|CastToBP_SaveGame_Skater _returnvalue_2))))
    (Variables|Persistence|SetLevelsUnlocked (Variables|/Game/Systems/BP_SaveGame_Skater.BP_SaveGame_Skater_C|GetLevelsUnlocked _output_get))
    (Variables|Persistence|SetTotalTimePlayed (Variables|/Game/Systems/BP_SaveGame_Skater.BP_SaveGame_Skater_C|GetTotalTimePlayed _output_get))
    (Variables|Persistence|SetLevelTimePlayed (Variables|/Game/Systems/BP_SaveGame_Skater.BP_SaveGame_Skater_C|GetLevelTimePlayed _output_get))
    (Variables|Persistence|SetLevelHighScore (Variables|/Game/Systems/BP_SaveGame_Skater.BP_SaveGame_Skater_C|GetLevelHighScore _output_get))
    (else
      (bind _returnvalue_3 (SaveGame|CreateSaveGameObject "/Game/Systems/BP_SaveGame_Skater.BP_SaveGame_Skater_C"))
      (Variables|Internal|SetSaveGameFile _returnvalue_3))))