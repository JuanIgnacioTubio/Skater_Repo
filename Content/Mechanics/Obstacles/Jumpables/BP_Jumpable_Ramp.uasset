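; BP_Jumpable_Ramp is a ramp obstacle that reports a player's jump interactions to the overlapping actor through interface-style messages.
; Its Box trigger sends an enter message on overlap begin, and a leave message carrying its ScoreValue on overlap end.
; Its StaticMesh sends a hit message when struck, leaving the scoring and reaction logic to the receiving actor.
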(event OnComponentBeginOverlap(Box)
  (params (OverlappedComponent :type Primitive%20Component%20Object%20Reference) (OtherActor :type Actor%20Object%20Reference) (OtherComp :type Primitive%20Component%20Object%20Reference) (OtherBodyIndex :type Integer) (bFromSweep :type Boolean) (SweepResult :type Hit%20Result%20Structure%20%28by%20ref%29))
  (Class|BPIScoring|JumpableEnterCollision(Message) OtherActor self))

(event OnComponentEndOverlap(Box)
  (params (OverlappedComponent :type Primitive%20Component%20Object%20Reference) (OtherActor :type Actor%20Object%20Reference) (OtherComp :type Primitive%20Component%20Object%20Reference) (OtherBodyIndex :type Integer))
  (Class|BPIScoring|JumpableLeaveCollision(Message) OtherActor (Variables|Default|GetScoreValue) self))

(event OnComponentHit(StaticMesh)
  (params (HitComponent :type Primitive%20Component%20Object%20Reference) (OtherActor :type Actor%20Object%20Reference) (OtherComp :type Primitive%20Component%20Object%20Reference) (NormalImpulse :type Vector :default "0, 0, 0") (Hit :type Hit%20Result%20Structure%20%28by%20ref%29))
  (Class|BPIScoring|JumpableHit(Message) OtherActor self))

(fn ConstructionScript
  (|CallParentFunction))