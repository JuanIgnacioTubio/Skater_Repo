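; Player character that switches between normal movement and a skating mode, with a pause toggle.
; Toggling skating swaps Enhanced Input mapping contexts and notifies the AnimInstance, while move input becomes acceleration and yaw steering.
; Tick sets clamped forward velocity and line-traces ahead for obstacles.
; A hit stops skating, knocks the player back, plays a falling montage with input disabled, then blinks the mesh before restoring control.
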(event Custom|CheckForUpcomingWall
  (bind _capsulecomponent (Variables|Default|GetCapsuleComponent))
  (bind _returnvalue (Transformation|GetWorldLocation _capsulecomponent))
  (bind _returnvalue_2 (Collision|LineTraceForObjects _returnvalue (+ _returnvalue (* (Math|Vector|GetForwardVector _capsulecomponent) (Math|Float|MakeLiteralFloat 75.0))) (Utilities|Array|MakeArray "ObjectTypeQuery1" "ObjectTypeQuery2" "ObjectTypeQuery3" "ObjectTypeQuery4") false 0 "None"))
  (if _returnvalue_2
    (CallFunction|PlayerCrash)))

(event Custom|ForceStopSkating
  (Variables|Default|SetbSkating false)
  (Development|PrintString (Utilities|String|Append "Skating Mode :" (Utilities|String|ToString(Boolean) (Variables|Default|GetbSkating))))
  (CallFunction|SwitchMappingContext (Variables|Default|GetbSkating))
  (Class|BPIAnimUpdates|UpdateMovementMode(Message) (Components|SkeletalMesh|GetAnimInstance (Variables|Character|GetMesh)) (Variables|Default|GetbSkating)))

(event Custom|PlayerCrash
  (CallFunction|ForceStopSkating)
  (Variables|/Script/Engine.MovementComponent|SetVelocity (Variables|Character|GetCharacterMovement) "0, 0, 0")
  (Character|LaunchCharacter (* (Math|Vector|GetForwardVector (Variables|Default|GetCapsuleComponent)) (* (Variables|Movement|GetSkatingSpeed) -0.4)) true false)
  (bind _notifyname (Animation|Montage|PlayMontage (Variables|Character|GetMesh) "/Game/Characters/Skater/Animations/AM_Player_FallingDown.AM_Player_FallingDown")
    (:then
      (Input|DisableInput (.AsPlayer%20Controller (Utilities|Casting|CastToPlayerController (Pawn|GetController)))))
    (:OnNotifyBegin
      (switch name _notifyname
        (:BeginFade
          (CallFunction|CrashFadeMesh)
          (bind _returnvalue (Utilities|Time|SetTimerbyEvent (delegate Custom|CrashFadeMesh) 0.3 true))
          (Variables|Animation|SetCrashFadeTimer _returnvalue))))))

(event Custom|CrashFadeMesh
  (Rendering|SetVisibility (Variables|Character|GetMesh) false true)
  (bind _result (Math|Integer|IncrementInt (Variables|Animation|GetCrashFadeCounter))
    (:%20%20
      (if (>= _result 3)
        (Utilities|Time|ClearandInvalidateTimerbyHandle (Variables|Animation|GetCrashFadeTimer))
        (Variables|Animation|SetCrashFadeCounter 0)
        (Utilities|FlowControl|Delay 0.15)
        (Rendering|SetVisibility (Variables|Character|GetMesh) true true)
        (Input|EnableInput (.AsPlayer%20Controller (Utilities|Casting|CastToPlayerController (Pawn|GetController))))
        (else
          (Utilities|FlowControl|Delay 0.15)
          (Rendering|SetVisibility (Variables|Character|GetMesh) true true))))))

(event Custom|SwitchMappingContext
  (params (bSkating :type Boolean))
  (bind _self self)
  (bind _self_2 self)
  (if bSkating
    (Input|RemoveMappingContext _self_2 "/Game/Systems/Input/IMC_Default.IMC_Default" (Utilities|Struct|MakeModifyContextOptions true false))
    (Input|AddMappingContext _self_2 "/Game/Systems/Input/IMC_Skating.IMC_Skating" 0 "(bIgnoreAllPressedKeysUntilRelease=True,bForceImmediately=False)")
    (else
      (Input|RemoveMappingContext _self "/Game/Systems/Input/IMC_Skating.IMC_Skating" (Utilities|Struct|MakeModifyContextOptions true false))
      (Input|AddMappingContext _self "/Game/Systems/Input/IMC_Default.IMC_Default" 0 "(bIgnoreAllPressedKeysUntilRelease=True,bForceImmediately=False)")))
  (Development|PrintString (select (.ReturnValue (Class|EnhancedInputSubsystemInterface|HasMappingContext (PlayerController|LocalPlayerSubsystems|GetEnhancedInputLocalPlayerSubsystem (Variables|Default|GetPlayerController)) "/Game/Systems/Input/IMC_Default.IMC_Default")) "Has Default Context" "Has Skating Context")))

(event EventBeginPlay
  (Variables|Default|SetPlayerController (.AsPlayer%20Controller (Utilities|Casting|CastToPlayerController (Pawn|GetController)))))

(event EventPause
  (if (Variables|Default|GetbPaused)
    (bind _output_get (Variables|Default|SetbPaused false))
    (Development|PrintString (Utilities|String|Append "Paused :" (Utilities|String|ToString(Boolean) _output_get)))
    (Game|SetGamePaused _output_get)
    (else
      (bind _output_get_2 (Variables|Default|SetbPaused true))
      (Development|PrintString (Utilities|String|Append "Paused :" (Utilities|String|ToString(Boolean) _output_get_2)))
      (Game|SetGamePaused _output_get_2))))

(event EventChangeMovementMode
  (if (Variables|Default|GetbSkating)
    (Variables|Default|SetbSkating false)
    (else
      (Variables|Movement|SetSkatingSpeed (Math|Vector|VectorLength (Variables|/Script/Engine.MovementComponent|GetVelocity (Variables|Character|GetCharacterMovement))))
      (Variables|Default|SetbSkating true)))
  (Development|PrintString (Utilities|String|Append "Skating Mode :" (Utilities|String|ToString(Boolean) (Variables|Default|GetbSkating))))
  (CallFunction|SwitchMappingContext (Variables|Default|GetbSkating))
  (Class|BPIAnimUpdates|UpdateMovementMode(Message) (Components|SkeletalMesh|GetAnimInstance (Variables|Character|GetMesh)) (Variables|Default|GetbSkating)))

(event EventMove
  (params (Value :type Input%20Action%20Value%20Structure%20%28by%20ref%29))
  (bind (_x _y) (Class|EnhancedInputLibrary|BreakInputActionValue Value))
  (if (Variables|Default|GetbSkating)
    (Variables|Movement|SetSkatingAcceleration (* _y 5.0))
    (Class|BPIAnimUpdates|SetAccelerating(Message) (Components|SkeletalMesh|GetAnimInstance (Variables|Character|GetMesh)) (> _y 0.0))
    (Transformation|AddWorldRotation (Variables|Default|GetCapsuleComponent) (Math|Rotator|MakeRotator 0.0 0.0 _x) false false)
    (else
      (|CallParentFunction Value))))

(event EventTick
  (params (DeltaSeconds :type Float%20%28single-precision%29))
  (if (Variables|Default|GetbSkating)
    (bind _output_get (Variables|Movement|SetSkatingSpeed (Math|Float|Clamp(Float) (+ (/ (Variables|Movement|GetSkatingAcceleration) DeltaSeconds) (Variables|Movement|GetSkatingSpeed)) 0.0 1.2e+03)))
    (Variables|/Script/Engine.MovementComponent|SetVelocity (Variables|Character|GetCharacterMovement) (* (Math|Vector|GetForwardVector (Variables|Default|GetCapsuleComponent)) _output_get))
    (CallFunction|CheckforUpcomingWall)))

(fn ConstructionScript)