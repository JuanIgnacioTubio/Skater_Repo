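; BP_Rail is a rail obstacle actor built around a single spline mesh component.
; The construction script shapes the mesh as a fixed-length segment along the root's forward vector, with equal start and end tangents.
; The start position comes from the root's world location, scaled unevenly per axis.
; Overlapping the mesh only prints the other actor's name, with no further rail behavior.
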(event OnComponentBeginOverlap(SplineMesh)
  (params (OverlappedComponent :type Primitive%20Component%20Object%20Reference) (OtherActor :type Actor%20Object%20Reference) (OtherComp :type Primitive%20Component%20Object%20Reference) (OtherBodyIndex :type Integer) (bFromSweep :type Boolean) (SweepResult :type Hit%20Result%20Structure%20%28by%20ref%29))
  (Development|PrintString (Utilities|GetDisplayName OtherActor)))

(fn ConstructionScript
  (bind _defaultsceneroot (Variables|Default|GetDefaultSceneRoot))
  (bind _defaultsceneroot_2 (Variables|Default|GetDefaultSceneRoot))
  (bind _returnvalue (Math|Vector|GetForwardVector _defaultsceneroot))
  (bind _returnvalue_2 (Transformation|GetWorldLocation _defaultsceneroot_2))
  (bind _returnvalue_3 (* _returnvalue_2 "1.000000,10.000000,10.000000"))
  (bind _returnvalue_4 (* _returnvalue "100.000000,100.000000,100.000000"))
  (SplineMesh|SetStartandEnd (Variables|Default|GetSplineMesh) _returnvalue_3 _returnvalue_4 (+ _returnvalue_3 (* (Math|Vector|GetForwardVector (Variables|Default|GetDefaultSceneRoot)) "200.000000,200.000000,200.000000")) _returnvalue_4 true :!class /Script/Engine.SplineMeshComponent))