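; Player character that toggles between walking and skateboarding, swapping camera boom, input mapping context and controller state.
; Skating drives velocity along capsule forward with curve-based turning, charged ollies and a forward trace that triggers crash knockback and mesh blinking.
; Jumped obstacles feed a timed combo: repeats yield diminishing points and time, unique obstacles multiply the score, and crashing halves it.
; Also handles pausing and reports playtime and high scores to the GameInstance.
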(event Custom|StopTickingTime
  (Utilities|Time|PauseTimerbyHandle (Variables|Internal|GetTimeTickTimer)))

(event Custom|ForceStopSkating
  (Variables|Movement|SetbSkating false)
  (CallFunction|DisableModeChange)
  (CallFunction|SetCameraMode (not (Variables|Movement|GetbSkating)))
  (CallFunction|SwitchMappingContext (Variables|Movement|GetbSkating))
  (Class|BPIAnimUpdates|UpdateMovementMode(Message) (Components|SkeletalMesh|GetAnimInstance (Variables|Character|GetMesh)) (Variables|Movement|GetbSkating)))

(event Custom|BeginTickingTime
  (if (Utilities|Time|IsValidTimerHandle (Variables|Internal|GetTimeTickTimer))
    (Utilities|Time|UnpauseTimerbyHandle (Variables|Internal|GetTimeTickTimer))
    (else
      (bind _returnvalue (Utilities|Time|SetTimerbyEvent (delegate Custom|TimeSecondTick) 1.0 true))
      (Variables|Internal|SetTimeTickTimer _returnvalue))))

(event Custom|ChangePauseVisibility
  (params (bPaused :type Boolean))
  (Default|ChangePauseVisibility (Variables|Internal|GetPlayerController) bPaused))

(event Custom|ReEnableModeChange
  (Variables|Movement|SetbCanChangeMode true))

(event Custom|DisableModeChange
  (Variables|Movement|SetbCanChangeMode false)
  (Utilities|Time|SetTimerbyEvent (delegate Custom|ReEnableModeChange) 0.2))

(event Custom|TimeSecondTick
  (Default|TickTimePlayed (Variables|Internal|GetGameInstance) 1.0))

(event Custom|SetCameraMode
  (params (bControllable :type Boolean))
  (if bControllable
    (Transformation|AttachComponentToComponent (Variables|Default|GetFollowCamera) (Variables|Default|GetCameraBoom) "None" "SnapToTarget" "SnapToTarget" "KeepRelative" true)
    (else
      (Transformation|AttachComponentToComponent (Variables|Default|GetFollowCamera) (Variables|Default|GetFixedCameraBoom) "None" "SnapToTarget" "SnapToTarget" "KeepRelative" true))))

(event EventBeginPlay
  (Variables|Internal|SetPlayerController (.AsBP%20Player%20Controller%20Skater (Utilities|Casting|CastToBP_PlayerController_Skater (Pawn|GetController))))
  (Variables|Internal|SetGameInstance (.AsBP%20Game%20Instance%20Skater (Utilities|Casting|CastToBP_GameInstance_Skater (Game|GetGameInstance))))
  (CallFunction|BeginTickingTime))

(event EventStopAccelerating
  (Class|BPIAnimUpdates|SetAccelerating(Message) (Components|SkeletalMesh|GetAnimInstance (Variables|Character|GetMesh)) false)
  (Variables|Movement|SetSkatingAcceleration 0.0))

(event EventPause
  (if (Variables|Internal|GetbPaused)
    (Variables|Internal|SetbPaused false)
    (else
      (Variables|Internal|SetbPaused true)))
  (CallFunction|ChangePauseVisibility (Variables|Internal|GetbPaused))
  (Game|SetGamePaused (Variables|Internal|GetbPaused)))

(event EventChangeMovementMode
  (if (Variables|Movement|GetbCanChangeMode)
    (if (Variables|Movement|GetbSkating)
      (Default|SetStateWalking (Variables|Internal|GetPlayerController))
      (Variables|Movement|SetbSkating false)
      (else
        (Variables|Movement|SetSkatingSpeed (Math|Vector|VectorLength (Variables|/Script/Engine.MovementComponent|GetVelocity (Variables|Character|GetCharacterMovement))))
        (Variables|Movement|SetbSkating true)
        (Default|SetStateRiding (Variables|Internal|GetPlayerController))))
    (CallFunction|DisableModeChange)
    (CallFunction|SetCameraMode (not (Variables|Movement|GetbSkating)))
    (CallFunction|SwitchMappingContext (Variables|Movement|GetbSkating))
    (Class|BPIAnimUpdates|UpdateMovementMode(Message) (Components|SkeletalMesh|GetAnimInstance (Variables|Character|GetMesh)) (Variables|Movement|GetbSkating))))

(event EventMove
  (params (Value :type Input%20Action%20Value%20Structure%20%28by%20ref%29))
  (bind (_x _y) (Class|EnhancedInputLibrary|BreakInputActionValue Value))
  (if (Variables|Movement|GetbSkating)
    (Variables|Movement|SetSkatingAcceleration (* _y 5.0))
    (Class|BPIAnimUpdates|SetAccelerating(Message) (Components|SkeletalMesh|GetAnimInstance (Variables|Character|GetMesh)) true)
    (Transformation|AddWorldRotation (Variables|Default|GetCapsuleComponent) (Math|Rotator|MakeRotator 0.0 0.0 (* _x (CallFunction|CalculateTurningSpeed))) false false)
    (Transformation|SetWorldRotation (Variables|Default|GetCameraBoom) (Transformation|GetWorldRotation (Variables|Default|GetCapsuleComponent)) false false)
    (else
      (|CallParentFunction Value))))

(event EventResumeGame
  (Variables|Internal|SetbPaused false)
  (CallFunction|ChangePauseVisibility (Variables|Internal|GetbPaused))
  (Game|SetGamePaused (Variables|Internal|GetbPaused)))

(event EventTick
  (params (DeltaSeconds :type Float%20%28single-precision%29))
  (bind _charactermovement (Variables|Character|GetCharacterMovement))
  (if (Variables|Movement|GetbSkating)
    (bind _output_get (Variables|Movement|SetSkatingSpeed (Math|Float|Clamp(Float) (+ (/ (Variables|Movement|GetSkatingAcceleration) DeltaSeconds) (Variables|Movement|GetSkatingSpeed)) 0.0 (Variables|Movement|GetMaxSkatingSpeed))))
    (Variables|/Script/Engine.MovementComponent|SetVelocity _charactermovement (Math|Vector|MakeVector (.X (Math|Vector|BreakVector (* (Math|Vector|GetForwardVector (Variables|Default|GetCapsuleComponent)) _output_get))) (.Y (Math|Vector|BreakVector (* (Math|Vector|GetForwardVector (Variables|Default|GetCapsuleComponent)) _output_get))) (.Z (Math|Vector|BreakVector (Variables|/Script/Engine.MovementComponent|GetVelocity _charactermovement)))))
    (CallFunction|CheckforUpcomingWall)))

(event Custom|SwitchMappingContext
  (params (bSkating :type Boolean))
  (bind _playercontroller (Variables|Internal|GetPlayerController))
  (bind _returnvalue (PlayerController|LocalPlayerSubsystems|GetEnhancedInputLocalPlayerSubsystem _playercontroller))
  (if bSkating
    (Input|RemoveMappingContext _returnvalue "/Game/Systems/Input/IMC_Default.IMC_Default" (Utilities|Struct|MakeModifyContextOptions true false))
    (Input|AddMappingContext _returnvalue "/Game/Systems/Input/IMC_Skating.IMC_Skating" 0 "(bIgnoreAllPressedKeysUntilRelease=True,bForceImmediately=False)")
    (else
      (Input|RemoveMappingContext _returnvalue "/Game/Systems/Input/IMC_Skating.IMC_Skating" (Utilities|Struct|MakeModifyContextOptions false false))
      (Input|AddMappingContext _returnvalue "/Game/Systems/Input/IMC_Default.IMC_Default" 0 "(bIgnoreAllPressedKeysUntilRelease=True,bForceImmediately=False)"))))

(event Input|EnhancedActionEvents|EnhancedInputActionIA_SkateJump
  (params (ActionValue :type Boolean) (ElapsedSeconds :type Float%20%28double-precision%29) (TriggeredSeconds :type Float%20%28double-precision%29) (InputAction :type Input%20Action%20Object%20Reference :default "/Game/Systems/Input/Actions/IA_SkateJump.IA_SkateJump"))
  (:Started
    (if (not (AI|Components|NavMovement|IsFalling (Variables|Character|GetCharacterMovement)))
      (CallFunction|BeginOllieCrouch)))
  (:Canceled
    (if (not (AI|Components|NavMovement|IsFalling (Variables|Character|GetCharacterMovement))) :!label _label
      (CallFunction|ReleaseOllieCrouch)
      (CallFunction|SkateJump)))
  (:Completed
    (goto _label)))

(event EventLook
  (params (Value :type Input%20Action%20Value%20Structure%20%28by%20ref%29))
  (if (not (Variables|Movement|GetbSkating))
    (|CallParentFunction Value)))

(event Custom|SkateJump
  (Character|LaunchCharacter (Math|Vector|MakeVector 0.0 0.0 (Math|Float|Clamp(Float) (* (* (Variables|Movement|GetSkatingSpeed) 1.0) (Variables|Movement|GetJumpMult)) 3.5e+02 1e+03)) false false))

(event Custom|ChangeBoardVisibility
  (params (bShow :type Boolean))
  (Rendering|SetVisibility (Variables|Default|GetSkateBoard) bShow false))

(event Custom|CheckForUpcomingWall
  (bind _capsulecomponent (Variables|Default|GetCapsuleComponent))
  (bind _returnvalue (Transformation|GetWorldLocation _capsulecomponent))
  (bind _returnvalue_2 (Collision|LineTraceForObjects _returnvalue (+ _returnvalue (* (Math|Vector|GetForwardVector _capsulecomponent) (Math|Float|MakeLiteralFloat 75.0))) (Utilities|Array|MakeArray "ObjectTypeQuery1" "ObjectTypeQuery2" "ObjectTypeQuery3" "ObjectTypeQuery4") false 0 "None"))
  (if _returnvalue_2
    (CallFunction|PlayerCrash)))

(event Custom|CancelSmallJumpAnimation
  (Utilities|FlowControl|Sequence
    (:then_0
      (bind _angle (Timeline|SmallSkateJump Stop)
        (:Update
          (Transformation|SetRelativeRotation (Variables|Default|GetSkateBoard) (Math|Rotator|MakeRotator (+ _angle -9e+01) 0.0 8e+01) false false))))
    (:then_1
      (Transformation|SetRelativeRotation (Variables|Default|GetSkateBoard) (Math|Rotator|MakeRotator -9e+01 0.0 8e+01) false false))))

(event Custom|CancelSkateJumpAnimation
  (if (Audio|Components|Audio|IsPlaying (Variables|Default|GetSmallSkateJump))
    (CallFunction|CancelSmallJumpAnimation)
    (elif (Audio|Components|Audio|IsPlaying (Variables|Default|GetBigSkateJump))
      (CallFunction|CancelBigJumpAnimation))))

(event Custom|PlayerCrash
  (CallFunction|ForceStopSkating)
  (CallFunction|ResetScoringObstacles)
  (CallFunction|CancelCombo)
  (Variables|/Script/Engine.MovementComponent|SetVelocity (Variables|Character|GetCharacterMovement) "0, 0, 0")
  (Character|LaunchCharacter (* (Math|Vector|GetForwardVector (Variables|Default|GetCapsuleComponent)) (* (Variables|Movement|GetSkatingSpeed) -0.4)) true false)
  (bind _notifyname (Animation|Montage|PlayMontage (Variables|Character|GetMesh) "/Game/Characters/Skater/Animations/AM_Player_FallingDown.AM_Player_FallingDown")
    (:then
      (Input|DisableInput (.AsPlayer%20Controller (Utilities|Casting|CastToPlayerController (Pawn|GetController))))
      (Default|SetStateFalling (Variables|Internal|GetPlayerController)))
    (:OnNotifyBegin
      (switch name _notifyname
        (:BeginFade
          (CallFunction|CrashFadeMesh)
          (bind _returnvalue (Utilities|Time|SetTimerbyEvent (delegate Custom|CrashFadeMesh) 0.3 true))
          (Variables|Animation|SetCrashFadeTimer _returnvalue))))))

(event Custom|CrashFadeMesh
  (Rendering|SetVisibility (Variables|Character|GetMesh) false true)
  (bind _result (Math|Integer|IncrementInt (Variables|Animation|GetCrashFadeCounter))
    (:%20%20
      (if (>= _result 3)
        (Utilities|Time|ClearandInvalidateTimerbyHandle (Variables|Animation|GetCrashFadeTimer))
        (Variables|Animation|SetCrashFadeCounter 0)
        (Utilities|FlowControl|Delay 0.15)
        (Rendering|SetVisibility (Variables|Character|GetMesh) true true)
        (Input|EnableInput (.AsPlayer%20Controller (Utilities|Casting|CastToPlayerController (Pawn|GetController))))
        (Default|SetStateWalking (Variables|Internal|GetPlayerController))
        (else
          (Utilities|FlowControl|Delay 0.15)
          (Rendering|SetVisibility (Variables|Character|GetMesh) true true))))))

(event Custom|BigJumpAnimation
  (bind _angle (Timeline|BigSkateJump PlayFromStart)
    (:Update
      (Transformation|SetRelativeRotation (Variables|Default|GetSkateBoard) (Math|Rotator|MakeRotator (+ _angle -9e+01) 0.0 8e+01) false false))))

(event Custom|CancelBigJumpAnimation
  (Utilities|FlowControl|Sequence
    (:then_0
      (bind _angle (Timeline|BigSkateJump Stop)
        (:Update
          (Transformation|SetRelativeRotation (Variables|Default|GetSkateBoard) (Math|Rotator|MakeRotator (+ _angle -9e+01) 0.0 8e+01) false false))))
    (:then_1
      (Transformation|SetRelativeRotation (Variables|Default|GetSkateBoard) (Math|Rotator|MakeRotator -9e+01 0.0 8e+01) false false))))

(event Custom|BeginOllieCrouch
  (bind (_direction _alpha _jumpmult) (Timeline|Timeline PlayFromStart)
    (:Update
      (Class|BPIAnimUpdates|SetCrouchAlpha(Message) (Components|SkeletalMesh|GetAnimInstance (Variables|Character|GetMesh)) _alpha)
      (Variables|Movement|SetJumpMult _jumpmult))))

(event Custom|ReleaseOllieCrouch
  (Utilities|FlowControl|Sequence
    (:then_0
      (bind (_direction _alpha _jumpmult) (Timeline|Timeline Stop)
        (:Update
          (Class|BPIAnimUpdates|SetCrouchAlpha(Message) (Components|SkeletalMesh|GetAnimInstance (Variables|Character|GetMesh)) _alpha)
          (Variables|Movement|SetJumpMult _jumpmult))))
    (:then_1
      (Class|BPIAnimUpdates|ReleaseOllieCrouch(Message) (Components|SkeletalMesh|GetAnimInstance (Variables|Character|GetMesh))))))

(event Custom|SmallJumpAnimation
  (bind _angle (Timeline|SmallSkateJump PlayFromStart)
    (:Update
      (Transformation|SetRelativeRotation (Variables|Default|GetSkateBoard) (Math|Rotator|MakeRotator (+ _angle -9e+01) 0.0 8e+01) false false))))

(event Custom|ResetScoringObstacles
  (Utilities|Array|Clear (Variables|Scoring|GetScoringObstacles)))

(event Custom|BeginCombo
  (bind _maxcomboduration (Variables|Scoring|Combo|GetMaxComboDuration))
  (bind _returnvalue (Utilities|Time|SetTimerbyEvent (delegate Custom|EndCombo) _maxcomboduration))
  (Variables|Scoring|Combo|SetComboTimer _returnvalue)
  (Default|SetStateJumping (Variables|Internal|GetPlayerController))
  (Default|SetComboTimer (Variables|Internal|GetPlayerController) _maxcomboduration _maxcomboduration))

(event Custom|EndCombo
  (bind _keys (Utilities|Map|Keys (Variables|Scoring|GetScoredObstacles)))
  (Default|UpdateFinalComboScore (Variables|Internal|GetPlayerController) (* (Variables|Scoring|Combo|GetSingleComboScore) (Utilities|Array|Length _keys)) (Utilities|Array|Length _keys) false)
  (Default|SetLevelHighScore (Variables|Internal|GetGameInstance) (* (Variables|Scoring|Combo|GetSingleComboScore) (Utilities|Array|Length _keys)))
  (Variables|Scoring|SetTotalScore (+ (Variables|Scoring|GetTotalScore) (* (Variables|Scoring|Combo|GetSingleComboScore) (Utilities|Array|Length _keys))))
  (Variables|Scoring|Combo|SetSingleComboScore 0.0)
  (Utilities|Map|Clear (Variables|Scoring|GetScoredObstacles))
  (Default|SetStateRiding (Variables|Internal|GetPlayerController)))

(event Custom|CancelCombo
  (bind _keys (Utilities|Map|Keys (Variables|Scoring|GetScoredObstacles)))
  (if (and (Utilities|Array|IsValidIndex _keys) (> (Variables|Scoring|Combo|GetSingleComboScore) 0.0))
    (Default|UpdateFinalComboScore (Variables|Internal|GetPlayerController) (/ (* (Variables|Scoring|Combo|GetSingleComboScore) (Utilities|Array|Length _keys)) 2.0) (Utilities|Array|Length _keys) true)
    (Default|SetLevelHighScore (Variables|Internal|GetGameInstance) (/ (* (Variables|Scoring|Combo|GetSingleComboScore) (Utilities|Array|Length _keys)) 2.0))
    (Variables|Scoring|SetTotalScore (+ (Variables|Scoring|GetTotalScore) (/ (* (Variables|Scoring|Combo|GetSingleComboScore) (Utilities|Array|Length _keys)) 2.0)))
    (Variables|Scoring|Combo|SetSingleComboScore 0.0)
    (Utilities|Time|ClearandInvalidateTimerbyHandle (Variables|Scoring|Combo|GetComboTimer))
    (Utilities|Map|Clear (Variables|Scoring|GetScoredObstacles))
    (Default|SetStateRiding (Variables|Internal|GetPlayerController))))

(event Custom|ExtendCombo
  (params (Seconds :type Float%20%28double-precision%29))
  (bind _maxcomboduration (Variables|Scoring|Combo|GetMaxComboDuration))
  (Development|PrintString (Utilities|String|ToString(Float) Seconds))
  (bind _output_get (Variables|Scoring|Combo|SetRemainingComboTime (Math|Float|Clamp(Float) (+ (Utilities|Time|GetTimerRemainingTimebyHandle (Variables|Scoring|Combo|GetComboTimer)) Seconds) 0.0 _maxcomboduration)))
  (Development|PrintString (Utilities|String|ToString(Float) _output_get))
  (Utilities|Time|ClearandInvalidateTimerbyHandle (Variables|Scoring|Combo|GetComboTimer))
  (Default|SetComboTimer (Variables|Internal|GetPlayerController) _output_get _maxcomboduration)
  (bind _returnvalue (Utilities|Time|SetTimerbyEvent (delegate Custom|EndCombo) _output_get))
  (Variables|Scoring|Combo|SetComboTimer _returnvalue))

(event EventJumpableEnterCollision
  (params (ObstacleActor :type Actor%20Object%20Reference))
  (if (Variables|Movement|GetbSkating)
    (Utilities|Array|AddUnique (Variables|Scoring|GetScoringObstacles) ObstacleActor)))

(event EventJumpableLeaveCollision
  (params (ScoreValue :type Float%20%28double-precision%29) (ObstacleActor :type Actor%20Object%20Reference) (BonusTime :type Float%20%28double-precision%29))
  (if (Variables|Movement|GetbSkating)
    (if (Utilities|Array|ContainsItem (Variables|Scoring|GetScoringObstacles) ObstacleActor)
      (if (Utilities|Map|IsEmpty (Variables|Scoring|GetScoredObstacles))
        (CallFunction|BeginCombo)
        (else
          (CallFunction|ExtendCombo (CallFunction|CalculateBonusTime BonusTime ObstacleActor))))
      (Variables|Scoring|Combo|SetSingleComboScore (+ (CallFunction|CalculateAddedScore ScoreValue ObstacleActor) (Variables|Scoring|Combo|GetSingleComboScore)))
      (Utilities|Array|RemoveItem (Variables|Scoring|GetScoringObstacles) ObstacleActor)
      (if (Utilities|Map|Contains (Variables|Scoring|GetScoredObstacles) ObstacleActor)
        (Utilities|Map|Add (Variables|Scoring|GetScoredObstacles) ObstacleActor (+ (.Value (Utilities|Map|Find (Variables|Scoring|GetScoredObstacles) ObstacleActor)) 1))
        (else
          (Utilities|Map|Add (Variables|Scoring|GetScoredObstacles) ObstacleActor 1)))
      (bind _keys (Utilities|Map|Keys (Variables|Scoring|GetScoredObstacles)))
      (Default|UpdateCurrentComboScore (Variables|Internal|GetPlayerController) (Variables|Scoring|Combo|GetSingleComboScore) (Utilities|Array|Length _keys)))))

(event EventJumpableHit
  (params (ObstacleActor :type Actor%20Object%20Reference))
  (Utilities|Array|RemoveItem (Variables|Scoring|GetScoringObstacles) ObstacleActor))

(fn ConstructionScript)

(fn CalculateBonusTime
  (params (InitialValue :type Float%20%28double-precision%29) (JumpedActor :type Actor%20Object%20Reference))
  (bind _scoredobstacles (Variables|Scoring|GetScoredObstacles))
  (return (select (Utilities|Map|Contains _scoredobstacles JumpedActor) (/ InitialValue (.Value (Utilities|Map|Find _scoredobstacles JumpedActor))) InitialValue)))

(fn CalculateAddedScore
  (params (InitialValue :type Float%20%28double-precision%29) (JumpedActor :type Actor%20Object%20Reference))
  (bind _scoredobstacles (Variables|Scoring|GetScoredObstacles))
  (return (select (Utilities|Map|Contains _scoredobstacles JumpedActor) (/ InitialValue (.Value (Utilities|Map|Find _scoredobstacles JumpedActor))) InitialValue)))

(fn CalculateTurningSpeed
  (return (Math|Float|Clamp(Float) (* (Variables|Movement|GetBaseTurningSpeed) (Math|Curves|GetFloatValue (Variables|Movement|GetTurningCoefCurve) (/ (Variables|Movement|GetSkatingSpeed) (Variables|Movement|GetMaxSkatingSpeed)))) 1.0 1e+01)))