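; BP_HUD_Skater is a player HUD Blueprint that owns the on-screen widget for the skater.
; On BeginPlay it creates WBP_HUD_Skater for player controller 0, adds it to the viewport and initializes it.
; Walking, riding, jumping and falling state events are thin pass-throughs to the matching functions on that widget, which does the actual display work.
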(event Custom|SetStateFalling
  (Default|SetStateFalling (Variables|Default|GetHUDWidget)))

(event Custom|SetStateWalking
  (Default|SetStateWalking (Variables|Default|GetHUDWidget)))

(event Custom|SetStateRiding
  (Default|SetStateRiding (Variables|Default|GetHUDWidget)))

(event Custom|SetStateJumping
  (Default|SetStateJumping (Variables|Default|GetHUDWidget)))

(event EventBeginPlay
  (bind _returnvalue (UserInterface|CreateWidget "/Game/UI/WBP_HUD_Skater.WBP_HUD_Skater_C" (Game|GetPlayerController 0)))
  (bind _output_get (Variables|Default|SetHUDWidget _returnvalue))
  (UserInterface|Viewport|AddtoViewport _output_get 0)
  (Default|Initialize _output_get))

(event Collision|EventActorBeginOverlap
  (params (OtherActor :type Actor%20Object%20Reference)))

(event EventTick
  (params (DeltaSeconds :type Float%20%28single-precision%29)))

(fn ConstructionScript)